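; BP_Table is a table actor with two chair components that tracks which seats are occupied.
; The construction script fills parallel arrays of chairs and occupancy flags, both seats starting free.
; IsTableFree returns the first free seat index, or -1 when full.
; OcupySeat marks a seat taken and returns that chair's world location, while FreeSeat clears its flag.
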(event `self.ReceiveActorBeginOverlap`
  (params (OtherActor :type "Actor Object Reference")))

(fn `FreeSeat`
  (params (Index :type Integer))
  (`KismetArrayLibrary.Array_Set` (`self.IsOcc`) Index))

(fn `IsTableFree`
  (returns (IsFree :type Boolean) (Index :type Integer))
  (bind _isocc (`self.IsOcc`))
  (for _index (range (+ (`KismetArrayLibrary.Array_LastIndex` _isocc) 1))
    (if (not (`|GetArrayItem` _isocc _index))
      (return true _index)))
  (return false -1))

(fn `OcupySeat`
  (params (Index :type Integer))
  (returns (Cgahirlocation :type "Vector Structure"))
  (`KismetArrayLibrary.Array_Set` (`self.IsOcc`) Index true)
  (return (`SceneComponent.K2_GetComponentLocation` (`|GetArrayItem` (`self.Chairs`) Index))))

(fn `UserConstructionScript`
  (set `self.Chairs` (`|MakeArray` (`self.Chair`) (`self.Chair1`)))
  (set `self.IsOcc` (`|MakeArray` false false)))